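; Enemy character that patrols around its spawn point and chases the player's ThirdPersonCharacter when it sees one.
; Patrolling line-traces down from high Z at random offsets within RadiodeMovimiento, moves to the impact point via AIMoveTo, then waits and repeats on success.
; PawnSensing sightings change the walk speed and redirect AIMoveTo to the seen character, with no explicit return to patrol.
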(event `self.ReceiveBeginPlay`
  (set `self.ubicaciónInicial` (`self.K2_GetActorLocation`))
  (`self.Patrullar`))

(event `Patrullar`
  (bind (`_ubicacióninicial_x` `_ubicacióninicial_y`) (`KismetMathLibrary.BreakVector` (`self.ubicaciónInicial`)))
  (bind _returnvalue (+ (`KismetMathLibrary.RandomFloatInRange` (* (`self.RadiodeMovimiento`) -1.0) (`self.RadiodeMovimiento`)) `_ubicacióninicial_y`))
  (bind _returnvalue_2 (+ (`KismetMathLibrary.RandomFloatInRange` (* (`self.RadiodeMovimiento`) -1.0) (`self.RadiodeMovimiento`)) `_ubicacióninicial_x`))
  (bind _outhit (`KismetSystemLibrary.LineTraceSingle` :`Start` (`KismetMathLibrary.MakeVector` _returnvalue_2 _returnvalue 14000.0) :`End` (`KismetMathLibrary.MakeVector` _returnvalue_2 _returnvalue) :`TraceChannel` "TraceTypeQuery1" :`bIgnoreSelf` false :`DrawTime` 100.0 :!label _label))
  (`|AIMoveTo` self (`.ImpactPoint` (`GameplayStatics.BreakHitResult` _outhit)) null
    (:`OnSuccess`
      (`KismetSystemLibrary.Delay` 2.0)
      (goto _label))))

(event `Cambiar vcelocidadd`
  (params (Velocidad :type "Float (double-precision)"))
  (set `CharacterMovementComponent.MaxWalkSpeed` Velocidad (`self.CharacterMovement`)))

(event `self.PawnSensing.OnSeePawn`
  (params (Pawn :type "Pawn Object Reference"))
  (bind _asthird_person_character (cast `/Game/ThirdPersonBP/Blueprints/ThirdPersonCharacter` Pawn))
  (`self.Cambiar vcelocidadd` 350.0)
  (`|AIMoveTo` self (0.0 0.0 0.0) _asthird_person_character 20.0))

(fn `UserConstructionScript`)